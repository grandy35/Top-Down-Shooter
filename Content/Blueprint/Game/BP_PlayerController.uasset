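; Player controller that turns movement, fire and reload input into actions on the possessed BP_Character and its current weapon.
; Movement pushes the pawn along fixed world X and Y axes, independent of facing.
; Fire caches character, weapon and mesh, then checks ammo, reloading and readiness before firing with a montage, or plays a dry-fire sound when empty.
; Reload uses those cached references, reloading with a montage unless ammo equals the weapon's round count.
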(event EventBeginPlay)

(event EventTick
  (params (DeltaSeconds :type Float%20%28single-precision%29)))

(event Input|ActionEvents|InputActionReload
  (params (Key :type Key%20Structure :default "None"))
  (bind _current_weapon (Variables|Default|GetCurrent%20Weapon))
  (:Pressed
    (bind _returnvalue (Class|Weapon|GetWeaponRound _current_weapon))
    (if (not (== (Variables|/Script/TopDownShooter.Weapon|GetCurrentAmmo _current_weapon) _returnvalue))
      (Class|Weapon|Reloading _current_weapon)
      (Animation|Montage|PlayMontage (Variables|Default|GetMesh) (Class|Weapon|GetReloadAnimation _current_weapon)))))

(event Input|ActionEvents|InputActionFire
  (params (Key :type Key%20Structure :default "None"))
  (:Pressed
    (bind _asbp_character (Utilities|Casting|CastToBP_Character (Pawn|GetControlledPawn)))
    (Variables|Default|SetBP_CharacterRef _asbp_character)
    (Utilities|IsValid (Variables|/Script/TopDownShooter.TopDownShooterCharacter|GetCurrentWeapon _asbp_character)
      (:Is%20Valid
        (Variables|Default|SetCurrent%20Weapon (Variables|/Script/TopDownShooter.TopDownShooterCharacter|GetCurrentWeapon _asbp_character))
        (Variables|Default|SetMesh (Variables|/Script/Engine.Character|GetMesh _asbp_character))
        (if (<= (Variables|/Script/TopDownShooter.Weapon|GetCurrentAmmo (Variables|Default|GetCurrent%20Weapon)) 0)
          (Audio|PlaySound2D "/Game/TopDownCPP/Sound/SC_DryFire_Cue.SC_DryFire_Cue" 1.0 1.0 0.0 0 0)
          (elif (Math|Boolean|NotEqual(Boolean) (Variables|/Script/TopDownShooter.Weapon|GetbIsReloading (Variables|Default|GetCurrent%20Weapon)) true)
            (if (Variables|/Script/TopDownShooter.TopDownShooterCharacter|GetAimEnabled (Variables|Default|GetBP_CharacterRef))
              _
              (else
                _))
            (if (Class|Weapon|IsReadytoFire (Variables|Default|GetCurrent%20Weapon))
              (Class|Weapon|Fire (Variables|Default|GetCurrent%20Weapon))
              (Animation|Montage|PlayMontage (Variables|Default|GetMesh) (Class|Weapon|GetCurrentFireAnimation (Variables|Default|GetCurrent%20Weapon)))))))
      (:Is%20Not%20Valid
        (Development|PrintString "NotWeapon!!!!!" true true "(R=1.000000,G=0.027472,B=0.000000,A=1.000000)" 5.0)))))

(event Input|AxisEvents|InputAxisMoveForward
  (params (AxisValue :type Float%20%28single-precision%29))
  (Pawn|Input|AddMovementInput (Game|Player|GetPlayerPawn 0) "1.000000, 0, 0" AxisValue false))

(event Input|AxisEvents|InputAxisMoveRight
  (params (AxisValue :type Float%20%28single-precision%29))
  (Pawn|Input|AddMovementInput (Game|Player|GetPlayerPawn 0) "0,1.000000, 0" AxisValue false))

(fn ConstructionScript)