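; BP_Enterance01 is a door entrance that opens for BP_Character and carries it to the level TopDownShooter_LVL2.
; Overlapping TriggerDoor plays the OpenDoor timeline, which drives the static mesh's relative yaw to swing it open; nothing here closes it again.
; Overlapping PortalTrigger adds a WBP_FadeScreen widget, calls its FadeIn, waits through a short delay, then opens that level by name.
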(event OnComponentBeginOverlap(TriggerDoor)
  (params (OverlappedComponent :type Primitive%20Component%20Object%20Reference) (OtherActor :type Actor%20Object%20Reference) (OtherComp :type Primitive%20Component%20Object%20Reference) (OtherBodyIndex :type Integer) (bFromSweep :type Boolean) (SweepResult :type Hit%20Result%20Structure%20%28by%20ref%29))
  (Utilities|Casting|CastToBP_Character OtherActor)
  (bind _open (Timeline|OpenDoor Play)
    (:Update
      (Transformation|SetRelativeRotation (Variables|Default|GetStaticMeshComponent0) (Math|Rotator|MakeRotator 0.0 0.0 _open) false false))))

(event OnComponentBeginOverlap(PortalTrigger)
  (params (OverlappedComponent :type Primitive%20Component%20Object%20Reference) (OtherActor :type Actor%20Object%20Reference) (OtherComp :type Primitive%20Component%20Object%20Reference) (OtherBodyIndex :type Integer) (bFromSweep :type Boolean) (SweepResult :type Hit%20Result%20Structure%20%28by%20ref%29))
  (Utilities|Casting|CastToBP_Character OtherActor)
  (bind _returnvalue (UserInterface|CreateWidget "/Game/TopDownCPP/Maps/Widget/WBP_FadeScreen.WBP_FadeScreen_C"))
  (UserInterface|Viewport|AddtoViewport _returnvalue 0)
  (Default|Fadein _returnvalue)
  (Utilities|FlowControl|Delay 2.0)
  (Game|OpenLevel(byName) "TopDownShooter_LVL2"))

(event EventBeginPlay)

(event Collision|EventActorBeginOverlap
  (params (OtherActor :type Actor%20Object%20Reference)))

(event EventTick
  (params (DeltaSeconds :type Float%20%28single-precision%29)))

(fn ConstructionScript)